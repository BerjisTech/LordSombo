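; BP_Zone is an actor that marks out a zone with copies of a mesh placed along a spline.
; The construction script sets the chosen Mesh on an InstancedStaticMesh and adds one world-space instance at each spline point, matching its location and rotation.
; A showZone event repeats the same placement at runtime, adding instances without clearing existing ones.
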(event Custom|showZone
  (bind _spline (Variables|Default|GetSpline))
  (Components|StaticMesh|SetStaticMesh (Variables|Default|GetInstancedStaticMesh) (Variables|Default|Getmesh))
  (for _index (range 0 (- (Spline|GetNumberOfSplinePoints _spline) 1))
    (Components|InstancedStaticMesh|AddInstance (Variables|Default|GetInstancedStaticMesh) (Math|Transform|MakeTransform (Spline|GetLocationatSplinePoint _spline _index "World") (Spline|GetRotationatSplinePoint _spline _index "World") "1.000000,1.000000,1.000000") true)))

(event EventBeginPlay)

(event Collision|EventActorBeginOverlap
  (params (OtherActor :type Actor%20Object%20Reference)))

(event EventTick
  (params (DeltaSeconds :type Float%20%28single-precision%29)))

(fn ConstructionScript
  (bind _spline (Variables|Default|GetSpline))
  (Components|StaticMesh|SetStaticMesh (Variables|Default|GetInstancedStaticMesh) (Variables|Default|Getmesh))
  (for _index (range 0 (- (Spline|GetNumberOfSplinePoints _spline) 1))
    (Components|InstancedStaticMesh|AddInstance (Variables|Default|GetInstancedStaticMesh) (Math|Transform|MakeTransform (Spline|GetLocationatSplinePoint _spline _index "World") (Spline|GetRotationatSplinePoint _spline _index "World") "1.000000,1.000000,1.000000") true)))