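; AIPaths is a spline path actor that populates itself with AI-driven Nganya traffic.
; The construction script flanks each spline point with box components.
; Below a vehicle cap, it spawns vehicles at every seventh point near the player, passing the spline and a random speed limit to AIC_NPCDriverController.
; A cleanup pass destroys nearby driverless, non-NPC vehicles, then a delay restarts the spawn cycle.
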(event Custom|SpawnVehicles
  (Utilities|SpawnNPCVehicles
    (:Completed
      (Utilities|DespawnNPCVehicles
        (:true
          (Utilities|FlowControl|Delay (Variables|Default|GetSpawnDelay))
          (CallFunction|SpawnVehicles))))))

(event EventBeginPlay
  (CallFunction|SpawnVehicles))

(event Collision|EventActorBeginOverlap
  (params (OtherActor :type Actor%20Object%20Reference)))

(event EventTick
  (params (DeltaSeconds :type Float%20%28single-precision%29)))

(fn ConstructionScript
  (bind _spline (Variables|Default|GetSpline))
  (for _index (range 0 (Spline|GetNumberOfSplinePoints _spline))
    (AddComponent|AddBoxComponent false (Math|Transform|MakeTransform (+ (.location (Spline|GetTransformatSplinePoint _spline _index "Local" false)) (Class|SplineComponent|GetRightVectoratSplinePoint _spline _index "Local")) (.rotation (Spline|GetTransformatSplinePoint _spline _index "Local" false)) "5.000000,0.500000,5.000000"))
    (AddComponent|AddBoxComponent false (Math|Transform|MakeTransform (- (.location (Spline|GetTransformatSplinePoint _spline _index "Local" false)) (Class|SplineComponent|GetRightVectoratSplinePoint _spline _index "Local")) (.rotation (Spline|GetTransformatSplinePoint _spline _index "Local" false)) "5.000000,0.500000,5.000000"))))