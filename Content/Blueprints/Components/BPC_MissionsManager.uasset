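; Player character component that runs timed missions, currently a single Arrival mission to meet Gabby, though its ChooseMission call is disconnected.
; BeginPlay caches sibling UI, money, interaction, save and radio components; ChooseMission maps the saved mission to Arrival.
; Arrival spawns a landscape-aligned marker at an offset from the player, then a one-second Delay loop checks distance against the time limit and updates the location pointer.
; Pass or fail shows a brief alert widget.
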(event EventBeginPlay
  (Utilities|SetPlayerData))

(event EventTick
  (params (DeltaSeconds :type Float%20%28single-precision%29)))