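; UI manager component that creates and toggles the player's HUD, direction pointer, phone, main menu and purchase screens.
; BeginPlay creates the HUD or prunes duplicates, then rebuilds the navigation pointer, which the navigationUI event can also refresh.
; FlipFlops on phone and menu input actions and hardcoded J/H keys open and close widgets, finding them by class for removal.
; Cursor visibility follows each screen; menu and purchase screens also pause the game.
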(event Custom|CreateHUD
  (bind _foundwidgets (Widget|GetAllWidgetsOfClass "/LordSombo/Blueprints/UI/WBP_PlayerHUD.WBP_PlayerHUD_C" false))
  (if (> (Utilities|Array|Length _foundwidgets) 0)
    (if (> (Utilities|Array|Length _foundwidgets) 1)
      (for (_array_element _array_index) _foundwidgets
        (if (> _array_index 0)
          (Widget|RemovefromParent _array_element)
          (else
            (bind _output_get (Variables|Default|SetPlayerHUD _array_element))
            (Widget|RemovefromParent _output_get)
            (UserInterface|Viewport|AddtoViewport _output_get 0)))))
    (else
      (bind _returnvalue (UserInterface|CreateWidget "/LordSombo/Blueprints/UI/WBP_PlayerHUD.WBP_PlayerHUD_C" (Game|GetPlayerController 0)))
      (bind _output_get_2 (Variables|Default|SetPlayerHUD _returnvalue))
      (UserInterface|Viewport|AddtoPlayerScreen _output_get_2))))

(event Custom|navigationUI
  (Utilities|NavigationPointer))

(event Input|EnhancedActionEvents|EnhancedInputActionIA_Phone
  (params (ActionValue :type Boolean) (ElapsedSeconds :type Float%20%28double-precision%29) (TriggeredSeconds :type Float%20%28double-precision%29) (InputAction :type Input%20Action%20Object%20Reference :default "/LordSombo/Blueprints/Input/IA_Phone.IA_Phone"))
  (:Started
    (Utilities|FlowControl|FlipFlop
      (:A
        (Utilities|ShowPhone))
      (:B
        (Utilities|HidePhone)))))

(event Input|EnhancedActionEvents|EnhancedInputActionIA_Menu
  (params (ActionValue :type Boolean) (ElapsedSeconds :type Float%20%28double-precision%29) (TriggeredSeconds :type Float%20%28double-precision%29) (InputAction :type Input%20Action%20Object%20Reference :default "/LordSombo/Blueprints/Input/IA_Menu.IA_Menu"))
  (:Started
    (Utilities|FlowControl|FlipFlop
      (:A
        (Utilities|ShowMainMenu))
      (:B
        (Utilities|HideMainMenu)))))

(event EventBeginPlay
  (CallFunction|CreateHUD)
  (Utilities|NavigationPointer))

(event EventTick
  (params (DeltaSeconds :type Float%20%28single-precision%29)))

(event Input|KeyboardEvents|J
  (params (Key :type Key%20Structure))
  (bind _returnvalue (Game|GetPlayerController 0))
  (:Pressed
    (Utilities|FlowControl|FlipFlop
      (:A
        (bind _returnvalue_2 (UserInterface|CreateWidget "/LordSombo/Blueprints/UI/WBP_VehiclePurchase.WBP_VehiclePurchase_C" _returnvalue))
        (UserInterface|Viewport|AddtoViewport _returnvalue_2 0)
        (Variables|/Script/Engine.PlayerController|SetbShowMouseCursor _returnvalue true)
        (Game|SetGamePaused true))
      (:B
        (bind _foundwidgets (Widget|GetAllWidgetsOfClass "/LordSombo/Blueprints/UI/WBP_VehiclePurchase.WBP_VehiclePurchase_C" true))
        (for _array_element _foundwidgets
          (Widget|RemovefromParent _array_element)
          (Variables|/Script/Engine.PlayerController|SetbShowMouseCursor _returnvalue false)
          (Game|SetGamePaused false))))))

(event Input|KeyboardEvents|H
  (params (Key :type Key%20Structure))
  (bind _returnvalue (Game|GetPlayerController 0))
  (:Pressed
    (Utilities|FlowControl|FlipFlop
      (:A
        (bind _returnvalue_2 (UserInterface|CreateWidget "/LordSombo/Blueprints/UI/WBP_PropertyPurchase.WBP_PropertyPurchase_C" _returnvalue))
        (UserInterface|Viewport|AddtoViewport _returnvalue_2 0)
        (Variables|/Script/Engine.PlayerController|SetbShowMouseCursor _returnvalue true)
        (Game|SetGamePaused true))
      (:B
        (bind _foundwidgets (Widget|GetAllWidgetsOfClass "/LordSombo/Blueprints/UI/WBP_PropertyPurchase.WBP_PropertyPurchase_C" true))
        (for _array_element _foundwidgets
          (Widget|RemovefromParent _array_element)
          (Variables|/Script/Engine.PlayerController|SetbShowMouseCursor _returnvalue false)
          (Game|SetGamePaused false))))))