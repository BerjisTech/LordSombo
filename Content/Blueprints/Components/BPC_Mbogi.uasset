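; BPC_Mbogi is a component that lets the player mark out territory and save it as a named zone.
; CapsLock spawns a landscape-aligned marker at the pawn's transform.
; Left Ctrl turns all markers in the world into a closed-loop BP_Zone spline, destroying them and displaying the zone.
; The spline points and a username-plus-random-float name form a zone record, which is added to the owner's BPC_SaveLoad and saved.
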(event Custom|GenerateZone
  (bind _returnvalue (Game|Player|GetPlayerPawn 0))
  (bind _locationpoints (Variables|Default|GetlocationPoints))
  (bind _outactors (Actor|GetAllActorsOfClass "/LordSombo/Blueprints/Actors/BP_TeritoryMarker.BP_TeritoryMarker_C"))
  (if (not (Utilities|Array|IsEmpty _outactors))
    (bind _returnvalue_2 (Game|SpawnActorfromClass "/LordSombo/Blueprints/Actors/BP_Zone.BP_Zone_C" (Transformation|GetActorTransform (Utilities|Array|Get(acopy) _outactors)) "AlwaysSpawn" "MultiplyWithRoot" _returnvalue _returnvalue))
    (Spline|SetClosedLoop (Variables|/LordSombo/Blueprints/Actors/BP_Zone.BP_Zone_C|GetSpline _returnvalue_2) false true)
    (for _array_element _outactors
      (Spline|AddSplinePoint (Variables|/LordSombo/Blueprints/Actors/BP_Zone.BP_Zone_C|GetSpline _returnvalue_2) (Transformation|GetActorLocation _array_element) "World" true)
      (Actor|DestroyActor _array_element))
    (CallFunction|PrepareSplineforAlignment _returnvalue_2)
    (Spline|SetClosedLoop (Variables|/LordSombo/Blueprints/Actors/BP_Zone.BP_Zone_C|GetSpline _returnvalue_2) true true)
    (Default|ShowZone _returnvalue_2)
    (for _index (range 0 (- (Spline|GetNumberOfSplinePoints (Variables|/LordSombo/Blueprints/Actors/BP_Zone.BP_Zone_C|GetSpline _returnvalue_2)) -1))
      (Utilities|Array|AddUnique (Variables|Default|GetlocationPoints) (Spline|GetLocationatSplinePoint (Variables|/LordSombo/Blueprints/Actors/BP_Zone.BP_Zone_C|GetSpline _returnvalue_2) _index "World")))
    (Variables|Default|SetnewZone (Utilities|Struct|MakeStruct_MbogiZones (Utilities|String|StringToName (Utilities|String|Append (Utilities|Platform|GetPlatformUserName) "-" (Utilities|String|ToString(Float) (Math|Random|RandomFloat)))) _locationpoints 0))
    (Utilities|Array|Clear _locationpoints)))

(event Custom|markTeritory
  (params (SpawnTransform :type Transform))
  (bind _returnvalue (Game|Player|GetPlayerPawn 0))
  (bind _returnvalue_2 (Game|SpawnActorfromClass "/LordSombo/Blueprints/Actors/BP_TeritoryMarker.BP_TeritoryMarker_C" SpawnTransform "AlwaysSpawn" "MultiplyWithRoot" _returnvalue _returnvalue))
  (CallFunction|AligntoLandscape _returnvalue_2))

(event EventBeginPlay)

(event EventTick
  (params (DeltaSeconds :type Float%20%28single-precision%29)))

(event Input|KeyboardEvents|CapsLock
  (params (Key :type Key%20Structure))
  (:Pressed
    (CallFunction|MarkTeritory (Transformation|GetActorTransform (Game|Player|GetPlayerPawn 0)))))

(event Input|KeyboardEvents|LeftCtrl
  (params (Key :type Key%20Structure))
  (bind _returnvalue (Components|GetOwner))
  (bind _returnvalue_2 (Actor|GetComponentbyClass _returnvalue "/LordSombo/Blueprints/Components/BPC_SaveLoad.BPC_SaveLoad_C"))
  (:Pressed
    (CallFunction|GenerateZone)
    (Utilities|Array|AddUnique (Variables|/LordSombo/Blueprints/Components/BPC_SaveLoad.BPC_SaveLoad_C|GetZones _returnvalue_2) (Variables|Default|GetnewZone))
    (Default|SaveGame _returnvalue_2)))