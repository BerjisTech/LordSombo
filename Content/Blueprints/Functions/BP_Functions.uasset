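; Utility Blueprint that snaps actors and splines to the ground, with helpers for nearest-vector search and readable distance and speed text.
; PrepareSplineForAlignment rebuilds the actor's spline at GroundSnappingPrecision intervals, then line-traces each point against WorldStatic along HitDirection.
; Hit points get a Z-fighting offset, and the first also moves the actor.
; Actors without a spline fall back to AlignToLandscape, a single trace from above.
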(fn GetSplinePonts
  (params (Spline :type Spline%20Component%20Object%20Reference))
  (LocalVariables|SetSpline%20Length (Spline|GetSplineLength Spline))
  (Utilities|Array|Resize (LocalVariables|GetSpline%20Points%20Location) (+ (Math|Float|Round (/ (LocalVariables|GetSpline%20Length) (Math|Float|Min(Float) (Math|Float|Max(Float) (LocalVariables|GetGround%20Snapping%20Precision) 1e+02) (LocalVariables|GetSpline%20%20World%20Length)))) 1))
  (for _index (range 0 (Math|Float|Round (/ (LocalVariables|GetSpline%20Length) (Math|Float|Min(Float) (Math|Float|Max(Float) (LocalVariables|GetGround%20Snapping%20Precision) 1e+02) (LocalVariables|GetSpline%20%20World%20Length)))))
    (LocalVariables|SetIndex _index)
    (Utilities|Array|SetArrayElem (LocalVariables|GetSpline%20Points%20Location) (LocalVariables|GetIndex) (Spline|GetLocationatDistanceAlongSpline Spline (* _index (LocalVariables|GetGround%20Snapping%20Precision)) "World")))
  (Spline|ClearSplinePoints Spline true)
  (Spline|SetSplinePoints Spline (LocalVariables|GetSpline%20Points%20Location) "World" true)
  (return (LocalVariables|GetSpline%20Points%20Location) (LocalVariables|GetSpline%20Length)))

(fn GetNearestVector
  (params (Vectors :type Array%20of%20Vectors) (ActorLocation :type Vector))
  (LocalVariables|SetClosest%20found%20vector (Utilities|Array|Get(acopy) Vectors))
  (for (_array_element _array_index) Vectors
    (if (!= _array_index 0)
      (if (< (Math|Vector|Distance(Vector) ActorLocation _array_element) (Math|Vector|Distance(Vector) (LocalVariables|GetClosest%20found%20vector) ActorLocation))
        (LocalVariables|SetClosest%20found%20vector _array_element))))
  (return (Math|Vector|Distance(Vector) ActorLocation _array_element) (LocalVariables|GetClosest%20found%20vector)))

(fn AligntoLandscape
  (params (Actor :type Actor%20Object%20Reference))
  (bind _returnvalue (Transformation|GetActorLocation Actor))
  (bind _returnvalue_2 (+ _returnvalue "0.000000,0.000000,500.000000"))
  (Transformation|SetActorLocation Actor _returnvalue_2 false true)
  (bind (_outhit _returnvalue_3) (Collision|LineTraceForObjects 0 _returnvalue_2 (+ _returnvalue_2 (* (LocalVariables|GetHit%20Direction) (LocalVariables|GetLine%20Trace%20Length))) (Utilities|Array|MakeArray "ObjectTypeQuery1") true (Utilities|Array|MakeArray Actor) "None"))
  (if _returnvalue_3
    (Transformation|SetActorLocation Actor (+ (.Location (Collision|BreakHitResult _outhit)) (Math|Vector|MakeVector 0.0 0.0 (LocalVariables|GetZ%20fighting%20Ground%20Offset))) false true)
    (return)
    (else
      (Development|PrintString 0 (Utilities|String|ToString(Boolean) _returnvalue_3)))))

(fn PrepareSplineforAlignment
  (params (actorToAling :type Actor%20Object%20Reference))
  (bind _returnvalue (Actor|GetComponentbyClass actorToAling "/Script/Engine.SplineComponent"))
  (LocalVariables|SetActor actorToAling)
  (Utilities|IsValid _returnvalue
    (:Is%20Valid
      (LocalVariables|SetSpline _returnvalue)
      (Utilities|FlowControl|Sequence
        (:then_0
          ;[1 1 1] Create and Stores Snapping points
          (bind _points (CallFunction|GetSplinePonts (LocalVariables|GetSpline)))
          (LocalVariables|SetSpline%20Points%20Location _points))
        (:then_1
          ;[1 1 1] Align points to the ground
          (for _index (range 0 (- (Spline|GetNumberOfSplinePoints (LocalVariables|GetSpline)) 1))
            (LocalVariables|SetCurrent%20Loop%20Index _index)
            (bind (_outhit _returnvalue_2) (Collision|LineTraceForObjects 0 (Utilities|Array|Get(acopy) (LocalVariables|GetSpline%20Points%20Location) (LocalVariables|GetCurrent%20Loop%20Index)) (+ (Utilities|Array|Get(acopy) (LocalVariables|GetSpline%20Points%20Location) (LocalVariables|GetCurrent%20Loop%20Index)) (* (LocalVariables|GetHit%20Direction) (LocalVariables|GetLine%20Trace%20Length))) (Utilities|Array|MakeArray "ObjectTypeQuery1") true 0 "None"))
            (if _returnvalue_2
              (if (== (LocalVariables|GetCurrent%20Loop%20Index) 0)
                (Transformation|SetActorLocation (LocalVariables|GetActor) (+ (.Location (Collision|BreakHitResult _outhit)) (Math|Vector|MakeVector 0.0 0.0 (LocalVariables|GetZ%20fighting%20Ground%20Offset))) false false))
              (Spline|SetLocationatSplinePoint (LocalVariables|GetSpline) (LocalVariables|GetCurrent%20Loop%20Index) (+ (.Location (Collision|BreakHitResult _outhit)) (Math|Vector|MakeVector 0.0 0.0 (LocalVariables|GetZ%20fighting%20Ground%20Offset))) "World" true)))
          (Utilities|Array|Clear (LocalVariables|GetSpline%20Points%20Location)))))
    (:Is%20Not%20Valid
      (CallFunction|AligntoLandscape actorToAling))))

(fn ReadableDistance
  (params (distance :type Float%20%28double-precision%29))
  (if (> distance 1e+02)
    (if (> distance 1e+05)
      (return (|kilometers distance))
      (else
        (return (|meters distance))))
    (else
      (return (|centimeters distance)))))

(fn Readablespeed
  (params (speed :type Float%20%28double-precision%29))
  (return (Utilities|String|Append (Utilities|String|ToString(Float) (* (/ speed 1e+02) 3.6)) "km/h")))