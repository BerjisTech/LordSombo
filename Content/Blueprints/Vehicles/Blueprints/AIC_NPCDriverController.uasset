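; AI controller that drives NPC Chaos vehicles along AIPaths road splines.
; A near-continuous delay loop steers toward a speed-scaled look-ahead point on the nearest spline and fans out seven line traces for obstacles.
; Trace distances and SpeedLimiter corner volumes set throttle, brake and speed limit, with sidestepping around vehicles and reversing when stuck.
; Tick checks wheel contact, destroying ungrounded, overlapping cars far from the player under a velocity-direction test.
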(event Custom|AI%20Drive
  (bind _vehiclepawn (Variables|Components|GetVehiclePawn))
  (Utilities|IsValid _vehiclepawn
    (:Is%20Valid
      (if (Variables|/LordSombo/Blueprints/Vehicles/Blueprints/bp_vehicle_base_pawn.bp_vehicle_base_pawn_C|Getis_npc _vehiclepawn)
        (bind _roads (CallFunction|GetRoads))
        (bind _steering (CallFunction|GetLane _roads))
        (CallFunction|Steer _steering)
        (CallFunction|LineTracer)
        (if (Variables|Trace|Check|GetisStuck?)
          (Utilities|Unstuck)
          (else
            (Utilities|VariableSpeedLimit
              (:Output
                (Utilities|SpeedbyDistanceOfHitActors (Variables|Trace|Data|GetFrontLineTraceHitResults) true)
                (Utilities|SpeedLimiter
                  (:UnderSpeedLimit
                    (CallFunction|SetInput 1.0 0.0))
                  (:OverSpeedLimit
                    (if (Math|Boolean|ORBoolean (Variables|Trace|Check|GetFrontLineTraceHitResults?) (Variables|Trace|Check|GetLeftFrontOffsetLineTraceHitResults?) (Variables|Trace|Check|GetRightFrontOffsetLineTraceHitResults?))
                      (Utilities|AdjustSpeeds)
                      (bind _turnindex (Utilities|GetCorner)
                        (:IsInCorner
                          (switch Utilities|FlowControl|Switch|SwitchonE_TurnIndex _turnindex
                            (:NewEnumerator0
                              (Utilities|SpeedLimiter
                                (:UnderSpeedLimit
                                  (CallFunction|SetInput 1.0 0.0))
                                (:OverSpeedLimit
                                  (CallFunction|SetInput 0.0 1.0))))
                            (:NewEnumerator1
                              (Utilities|SpeedLimiter
                                (:UnderSpeedLimit
                                  (CallFunction|SetInput 1.0 0.0))
                                (:OverSpeedLimit
                                  (CallFunction|SetInput 0.0 1.0))))))
                        (:IsNotInCorner
                          (bind _vehicle (Utilities|CasttoVehicleBase (Variables|Trace|Data|GetLeftFrontOffsetLineTraceHitResults))
                            (:CastSuccess
                              (Utilities|OtherVehicleDirection _vehicle
                                (:TowardsEachOther
                                  (CallFunction|Steer -1.0))
                                (:SameDirection
                                  (CallFunction|Steer 1.0))))
                            (:CastFailed
                              (bind _vehicle_2 (Utilities|CasttoVehicleBase (Variables|Trace|Data|GetFrontLineTraceHitResults))
                                (:CastSuccess
                                  (Utilities|SpeedbyDistanceOfHitActors (Variables|Trace|Data|GetFrontLineTraceHitResults) false)
                                  (Utilities|OtherVehicleDirection _vehicle_2
                                    (:TowardsEachOther
                                      (CallFunction|Steer -1.0))
                                    (:SameDirection
                                      (CallFunction|Steer 1.0))))
                                (:CastFailed
                                  (bind _vehicle_3 (Utilities|CasttoVehicleBase (Variables|Trace|Data|GetRightFrontOffsetLineTraceHitResults))
                                    (:CastSuccess
                                      (Utilities|OtherVehicleDirection _vehicle_3
                                        (:TowardsEachOther
                                          (CallFunction|Steer -1.0))
                                        (:SameDirection
                                          (CallFunction|Steer 1.0))))
                                    (:CastFailed
                                      (CallFunction|SetInput 0.0 (Math|Float|MapRangeClamped (.distance (Utilities|Array|Get(acopy) (Variables|Trace|Data|GetFrontLineTraceHitResults))) 0.0 (Variables|Trace|Control|Values|GetLineTraceRange) 1.0 0.0))))))))))
                      (else
                        (CallFunction|SetInput 1.0 0.0)))))))))))))

(event EventBeginPlay
  (Utilities|FlowControl|Delay 2.0)
  (Variables|Speed|SetActive%20Speed%20Limit (Variables|Speed|GetSpeed%20Limit))
  (bind _asbp_vehicle_base_pawn (Utilities|Casting|CastTobp_vehicle_base_pawn (Pawn|GetControlledPawn)))
  (bind _output_get (Variables|Components|SetVehiclePawn _asbp_vehicle_base_pawn))
  (Utilities|IsValid (Actor|GetComponentbyClass _output_get "/LordSombo/Blueprints/Components/BPC_Vehicle_Interaction.BPC_Vehicle_Interaction_C")
    (:Is%20Valid
      (Default|StartEngine (Actor|GetComponentbyClass _output_get "/LordSombo/Blueprints/Components/BPC_Vehicle_Interaction.BPC_Vehicle_Interaction_C")))
    (:Is%20Not%20Valid
      _))
  (if (Variables|/LordSombo/Blueprints/Vehicles/Blueprints/bp_vehicle_base_pawn.bp_vehicle_base_pawn_C|Getis_npc _output_get) :!label _label
    (Default|SetAIControllerParameters _asbp_vehicle_base_pawn)
    (CallFunction|AIDrive)
    (Utilities|FlowControl|Delay 0.0002)
    (goto _label)))

(event EventTick
  (params (DeltaSeconds :type Float%20%28single-precision%29))
  (bind _vehiclepawn (Variables|Components|GetVehiclePawn))
  (Utilities|IsValid _vehiclepawn
    (:Is%20Valid
      (if (Variables|/LordSombo/Blueprints/Vehicles/Blueprints/bp_vehicle_base_pawn.bp_vehicle_base_pawn_C|Getis_npc _vehiclepawn)
        (Utilities|MovingonGround?)))))

(fn ConstructionScript)

(fn GetCurrentCarSpeed
  (return (* (Vehicle|GetForwardSpeed (Variables|Default|GetVehicleMovementComponent)) 0.036)))

(fn GetLane
  (params (Spline :type Array%20of%20AI%20Paths%20Object%20References))
  (bind _vehiclepawn (Variables|Components|GetVehiclePawn))
  (bind _returnvalue (Transformation|GetActorLocation _vehiclepawn))
  (Utilities|IsValid (Variables|Default|Get_spline)
    (:Is%20Valid
      _)
    (:Is%20Not%20Valid
      (Variables|Default|Set_spline (Variables|/LordSombo/Blueprints/Actors/AIPaths.AIPaths_C|GetSpline (.AsAIPaths (Utilities|Casting|CastToAIPaths (.ReturnValue (Actor|FindNearestActor (Transformation|GetActorLocation (Variables|Components|GetVehiclePawn)) Spline))))))))
  (return (Math|Float|MapRangeClamped (.yaw (Math|Rotator|Delta(Rotator) (Math|Rotator|FindLookatRotation _returnvalue (Spline|FindLocationClosesttoWorldLocation (Variables|Default|Get_spline) (+ (* (Math|Vector|Normalize (Class|SplineComponent|FindTangentClosesttoWorldLocation (Variables|Default|Get_spline) (Transformation|GetActorLocation (Variables|Components|GetVehiclePawn)) "World")) (Math|Float|MapRangeClamped (CallFunction|GetCurrentCarSpeed) 2e+01 8e+01 5e+01 5e+02)) _returnvalue) "World")) (Transformation|GetActorRotation (Variables|Components|GetVehiclePawn)))) -9e+01 9e+01 -1.0 1.0)))

(fn GetRoads
  (bind _outactors (Actor|GetAllActorsOfClass "/LordSombo/Blueprints/Actors/AIPaths.AIPaths_C"))
  (return _outactors))

(fn Steer
  (params (Steering :type Float%20%28single-precision%29))
  (bind _returnvalue (* Steering -1.0))
  (bind _isstuck_ (Variables|Trace|Check|GetisStuck?))
  (bind _returnvalue_2 (Math|Float|SelectFloat _returnvalue Steering _isstuck_))
  (Class|ChaosVehicleMovementComponent|SetSteeringInput (Variables|Default|GetVehicleMovementComponent) _returnvalue_2)
  (if (!= _returnvalue_2 0.0)
    _))

(fn SetInput
  (params (Throttle :type Float%20%28single-precision%29) (Brake :type Float%20%28single-precision%29))
  (bind _vehiclemovementcomponent (Variables|Default|GetVehicleMovementComponent))
  (Class|ChaosVehicleMovementComponent|SetThrottleInput _vehiclemovementcomponent (Math|Float|SelectFloat -1.0 Throttle (Variables|Trace|Check|GetisStuck?)))
  (Class|ChaosVehicleMovementComponent|SetBrakeInput _vehiclemovementcomponent (Math|Float|SelectFloat 1.0 Brake (Variables|Trace|Check|GetisStuck?))))

(fn LineTracer
  (bind _frontlinetraceorigin (Variables|Default|GetfrontLineTraceOrigin))
  (bind _returnvalue (Transformation|GetWorldLocation _frontlinetraceorigin))
  (for _index (range 0 6)
    (LocalVariables|SetCurrent%20index _index)
    (bind (_outhits _returnvalue_2) (Class|KismetSystemLibrary|LineTraceMultiforObjects (Utilities|Select :Index (LocalVariables|GetCurrent%20index) :Option%200 _returnvalue :Option%201 _returnvalue :Option%202 (Transformation|GetWorldLocation (Variables|Default|GetLineTraceFrontLeftOffset)) :Option%203 _returnvalue :Option%204 (Transformation|GetWorldLocation (Variables|Default|GetLineTraceFrontRightOffset)) :Option%205 _returnvalue :Option%206 _returnvalue) (+ (Utilities|Select :Index (LocalVariables|GetCurrent%20index) :Option%200 _returnvalue :Option%201 _returnvalue :Option%202 (Transformation|GetWorldLocation (Variables|Default|GetLineTraceFrontLeftOffset)) :Option%203 _returnvalue :Option%204 (Transformation|GetWorldLocation (Variables|Default|GetLineTraceFrontRightOffset)) :Option%205 _returnvalue :Option%206 _returnvalue) (* (Math|Vector|RotateVectorAroundAxis (Math|Vector|GetForwardVector (Variables|Default|GetfrontLineTraceOrigin)) (Utilities|Select :Index (LocalVariables|GetCurrent%20index) :Option%200 -9e+01 :Option%201 -45.0 :Option%202 0.0 :Option%203 0.0 :Option%204 0.0 :Option%205 45.0 :Option%206 9e+01) "0.000000,0.000000,1.000000") (Variables|Trace|Control|Values|GetLineTraceRange))) (Utilities|Array|MakeArray "ObjectTypeQuery7" "ObjectTypeQuery5" "ObjectTypeQuery3" "ObjectTypeQuery1") true (Utilities|Array|MakeArray (Variables|Components|GetVehiclePawn)) "None" true))
    (bind _output_get (Variables|Trace|Data|SetOutHitObjects _outhits))
    (bind _output_get_2 (Variables|Trace|Check|SetLineTraceHit? _returnvalue_2))
    (switch int (LocalVariables|GetCurrent%20index)
      (:0
        (Variables|Trace|Data|SetLeftLineTraceHitResults _output_get)
        (Variables|Trace|Check|SetLeftLineTraceHitResults? _output_get_2))
      (:1
        (Variables|Trace|Data|SetLeftFrontLineTraceHitResults _output_get)
        (Variables|Trace|Check|SetLeftFrontLineTraceHitResults? _output_get_2))
      (:2
        (Variables|Trace|Data|SetLeftFrontOffsetLineTraceHitResults _output_get)
        (Variables|Trace|Check|SetLeftFrontOffsetLineTraceHitResults? _output_get_2))
      (:3
        (Variables|Trace|Data|SetFrontLineTraceHitResults _output_get)
        (Variables|Trace|Check|SetFrontLineTraceHitResults? _output_get_2))
      (:4
        (Variables|Trace|Data|SetRightFrontOffsetLineTraceHitResults _output_get)
        (Variables|Trace|Check|SetRightFrontOffsetLineTraceHitResults? _output_get_2))
      (:5
        (Variables|Trace|Data|SetRightFrontLineTraceHitResults _output_get))
      (:6
        (Variables|Trace|Data|SetRightLineTraceHitResults _output_get))))
  (return))